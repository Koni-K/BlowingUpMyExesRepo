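; First-person player character that switches between unarmed, for luring actors, and armed with a single-shot rocket launcher.
; A camera line trace drives the lure and its HUD prompt, while weapon state also decides whether the player can be detected.
; Fire montage notifies sequence reloading, rocket bone visibility and ammo updates.
; Movement includes sprint, jump, timeline head bob and aim zoom, with damage, death and weapon swaps messaged to HUD or game mode.
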(event Custom|WeaponSwap
  (bind _weapon (Variables|Default|GetWeapon))
  (bind _armrig (Variables|Default|GetArmRig))
  ;[0.15 0.15 0.15 0.5] Swap Weapons
  (switch Utilities|FlowControl|Switch|SwitchonE_HeldWeapon (Variables|Default|GetcurrentWeapon)
    (:NewEnumerator0
      (Rendering|SetVisibility _weapon false false)
      (Animation|Montage|PlayMontage _armrig "/Game/Art/SkeletalMesh/armRig/AM_EquipUnarmed.AM_EquipUnarmed"))
    (:NewEnumerator1
      (Rendering|SetVisibility _weapon true false)
      (Variables|Default|SetcanReload? false)
      (Animation|Montage|PlayMontage _armrig "/Game/Art/SkeletalMesh/armRig/AM_EquipArmed.AM_EquipArmed"))))

(event Custom|Die
  (Utilities|FlowControl|Sequence
    (:then_0
      (Utilities|FlowControl|DoOnce false
        (:Completed
          (Class|BPIGame|Lose(Message) (Game|GetGameMode)))))
    (:then_1
      (Rendering|SetVisibility (Variables|Default|GetArmRig) false true))))

(event Input|EnhancedActionEvents|EnhancedInputActionIA_Move
  (params (ActionValue :type Vector%202D%20Structure) (ElapsedSeconds :type Float%20%28double-precision%29) (TriggeredSeconds :type Float%20%28double-precision%29) (InputAction :type Input%20Action%20Object%20Reference :default "/Game/Systems/Player/Input/Actions/IA_Move.IA_Move"))
  (bind _tl_headbob (Variables|Default|GetTL_HeadBob))
  ;[0.15 0.15 0.15 0.5] Omnidirectional Movement
  (:Triggered
    (Pawn|Input|AddMovementInput (Transformation|GetActorForwardVector) (.x ActionValue) false)
    (Pawn|Input|AddMovementInput (Transformation|GetActorRightVector) (.y ActionValue) false))
  (:Started
    (Components|Timeline|PlayfromStart _tl_headbob))
  (:Completed
    (Audio|Components|Audio|Stop _tl_headbob)))

(event Input|EnhancedActionEvents|EnhancedInputActionIA_Look
  (params (ActionValue :type Vector%202D%20Structure) (ElapsedSeconds :type Float%20%28double-precision%29) (TriggeredSeconds :type Float%20%28double-precision%29) (InputAction :type Input%20Action%20Object%20Reference :default "/Game/Systems/Player/Input/Actions/IA_Look.IA_Look"))
  ;[0.15 0.15 0.15 0.5] Look
  (Pawn|Input|AddControllerPitchInput (* (.y ActionValue) -1.0))
  (Pawn|Input|AddControllerYawInput (.x ActionValue)))

(event Input|EnhancedActionEvents|EnhancedInputActionIA_Jump
  (params (ActionValue :type Boolean) (ElapsedSeconds :type Float%20%28double-precision%29) (TriggeredSeconds :type Float%20%28double-precision%29) (InputAction :type Input%20Action%20Object%20Reference :default "/Game/Systems/Player/Input/Actions/IA_Jump.IA_Jump"))
  ;[0.15 0.15 0.15 0.5] Launches the player in the air
  (Character|Jump))

(event Input|EnhancedActionEvents|EnhancedInputActionIA_Shoot
  (params (ActionValue :type Boolean) (ElapsedSeconds :type Float%20%28double-precision%29) (TriggeredSeconds :type Float%20%28double-precision%29) (InputAction :type Input%20Action%20Object%20Reference :default "/Game/Systems/Player/Input/Actions/IA_Shoot.IA_Shoot"))
  ;[0.15 0.15 0.15 0.5] Player will shoot the rocket launcher if Equipped
  (:Started
    (switch Utilities|FlowControl|Switch|SwitchonE_HeldWeapon (Variables|Default|GetcurrentWeapon)
      (:NewEnumerator1
        (if (and (Variables|Default|GetcanShoot) (> (Variables|Default|GetCurrentAmmo) 0))
          (Math|Integer|DecrementInt (Variables|Default|GetCurrentAmmo)
            (:%20%20
              (Class|BPIUI|UpdateLoadedAmmo(Message) (Variables|Components|GetUI))
              (Components|SkinnedMesh|HideBonebyName (Variables|Default|GetWeapon) "Rocket1" "PBO_None")
              (Variables|Default|SetcanShoot false)
              (Game|SpawnActorfromClass "/Game/Systems/Player/Rocket.Rocket_C" (Transformation|GetWorldTransform (Variables|Default|GetshootLoc)) "Undefined" "MultiplyWithRoot" 0 self)
              (Variables|Default|SetcanReload? true)
              (bind _notifyname (Animation|Montage|PlayMontage (Variables|Default|GetArmRig) "/Game/Art/SkeletalMesh/armRig/AM_Fire.AM_Fire")
                (:OnNotifyBegin
                  (CallFunction|RocketReloadNotify _notifyname))))))))))

(event Input|EnhancedActionEvents|EnhancedInputActionIA_Run
  (params (ActionValue :type Boolean) (ElapsedSeconds :type Float%20%28double-precision%29) (TriggeredSeconds :type Float%20%28double-precision%29) (InputAction :type Input%20Action%20Object%20Reference :default "/Game/Systems/Player/Input/Actions/IA_Run.IA_Run"))
  (bind _charactermovement (Variables|Character|GetCharacterMovement))
  ;[0.15 0.15 0.15 0.5] Run
  (:Started
    (Variables|/Script/Engine.CharacterMovementComponent|SetMaxWalkSpeed _charactermovement (Variables|Movement|GetsprintSpeed))
    (Variables|Default|SetRunPressed true))
  (:Completed
    (Variables|/Script/Engine.CharacterMovementComponent|SetMaxWalkSpeed _charactermovement (Variables|Movement|GetwalkSpeed))
    (Variables|Default|SetRunPressed false)))

(event Input|EnhancedActionEvents|EnhancedInputActionIA_Aim
  (params (ActionValue :type Boolean) (ElapsedSeconds :type Float%20%28double-precision%29) (TriggeredSeconds :type Float%20%28double-precision%29) (InputAction :type Input%20Action%20Object%20Reference :default "/Game/Systems/Player/Input/Actions/IA_Aim.IA_Aim"))
  (bind _tl_zoom (Variables|Default|GetTL_Zoom))
  ;[0.15 0.15 0.15 0.5] Aim
  (:Started
    (Audio|Components|Audio|Play _tl_zoom))
  (:Completed
    (Utilities|String|Reverse _tl_zoom)))

(event Input|EnhancedActionEvents|EnhancedInputActionIA_SwapWeapon
  (params (ActionValue :type Float%20%28double-precision%29) (ElapsedSeconds :type Float%20%28double-precision%29) (TriggeredSeconds :type Float%20%28double-precision%29) (InputAction :type Input%20Action%20Object%20Reference :default "/Game/Systems/Player/Input/Actions/IA_SwapWeapon.IA_SwapWeapon"))
  (bind _weapon (Variables|Default|GetWeapon))
  (bind _armrig (Variables|Default|GetArmRig))
  ;[0.15 0.15 0.15 0.5] Swap Weapons
  (:Started
    (bind _isa (Utilities|FlowControl|FlipFlop)
      (:A
        (Variables|Default|SetcurrentWeapon "NewEnumerator1"))
      (:B
        (Variables|Default|SetcurrentWeapon "NewEnumerator0")))
    (Class|BPIGame|SwitchedWeapon(Message) (Game|GetGameMode) _isa)
    (switch Utilities|FlowControl|Switch|SwitchonE_HeldWeapon (Variables|Default|GetcurrentWeapon)
      (:NewEnumerator0
        (Rendering|SetVisibility _weapon false false)
        (Animation|Montage|PlayMontage _armrig "/Game/Art/SkeletalMesh/armRig/AM_EquipUnarmed.AM_EquipUnarmed"))
      (:NewEnumerator1
        (Rendering|SetVisibility _weapon true false)
        (Variables|Default|SetcanReload? false)
        (Animation|Montage|PlayMontage _armrig "/Game/Art/SkeletalMesh/armRig/AM_EquipArmed.AM_EquipArmed")))))

(event Input|EnhancedActionEvents|EnhancedInputActionIA_Inspect
  (params (ActionValue :type Boolean) (ElapsedSeconds :type Float%20%28double-precision%29) (TriggeredSeconds :type Float%20%28double-precision%29) (InputAction :type Input%20Action%20Object%20Reference :default "/Game/Systems/Player/Input/Actions/IA_Inspect.IA_Inspect"))
  ;[0.15 0.15 0.15 0.5] Inspect Weapon
  (:Started
    (switch Utilities|FlowControl|Switch|SwitchonE_HeldWeapon (Variables|Default|GetcurrentWeapon)
      (:NewEnumerator1
        (Animation|Montage|PlayMontage (Variables|Default|GetArmRig) "/Game/Art/SkeletalMesh/armRig/AM_Inspect.AM_Inspect")))))

(event Input|EnhancedActionEvents|EnhancedInputActionIA_Reload
  (params (ActionValue :type Boolean) (ElapsedSeconds :type Float%20%28double-precision%29) (TriggeredSeconds :type Float%20%28double-precision%29) (InputAction :type Input%20Action%20Object%20Reference :default "/Game/Systems/Player/Input/Actions/IA_Reload.IA_Reload"))
  ;[0.15 0.15 0.15 0.5] Reload
  (:Started
    (if (Math|Boolean|ANDBoolean (not (Variables|Default|GetcanShoot)) (not (Variables|Default|GetcanReload?)) (Utilities|Enum|Equal(Enum) (Variables|Default|GetcurrentWeapon) "NewEnumerator1") (> (Variables|Default|GetCurrentAmmo) 0))
      (Variables|Default|SetcanReload? true)
      (bind _notifyname (Animation|Montage|PlayMontage (Variables|Default|GetArmRig) "/Game/Art/SkeletalMesh/armRig/AM_Fire.AM_Fire" 1.0 0.0 "Reload")
        (:OnNotifyBegin
          (CallFunction|RocketReloadNotify _notifyname))))))

(event Input|EnhancedActionEvents|EnhancedInputActionIA_Interact
  (params (ActionValue :type Boolean) (ElapsedSeconds :type Float%20%28double-precision%29) (TriggeredSeconds :type Float%20%28double-precision%29) (InputAction :type Input%20Action%20Object%20Reference :default "/Game/Systems/Player/Input/Actions/IA_Interact.IA_Interact"))
  ;[0.15 0.15 0.15 0.5] Lure
  (:Started
    (switch Utilities|FlowControl|Switch|SwitchonE_HeldWeapon (Variables|Default|GetcurrentWeapon)
      (:NewEnumerator0
        (bind (_hitactor _isvalid_) (CallFunction|LureTrace))
        (if _isvalid_
          (bind _result (Class|BPINPC|CanLure?(Message) _hitactor))
          (if _result
            (Class|BPINPC|Lure(Message) _hitactor self)
            (Animation|Montage|PlayMontage (Variables|Default|GetArmRig) "/Game/Art/SkeletalMesh/armRig/AM_Lure.AM_Lure")))))))

(event EventTick
  (params (DeltaSeconds :type Float%20%28single-precision%29))
  (bind _ui (Variables|Components|GetUI))
  ;[0.15 0.15 0.15 0.5] Tick
  (switch Utilities|FlowControl|Switch|SwitchonE_HeldWeapon (Variables|Default|GetcurrentWeapon)
    (:NewEnumerator0
      (bind (_hitactor _isvalid_) (CallFunction|LureTrace))
      (if _isvalid_
        (bind _result (Class|BPINPC|CanLure?(Message) _hitactor))
        (if _result
          (Class|BPIUI|AddLurePopup(Message) _ui)
          (else
            (Class|BPIUI|RemoveLurePopup(Message) _ui :!label _label)))
        (else
          (goto _label))))
    (:NewEnumerator1
      (Class|BPIUI|RemoveLurePopup(Message) (Variables|Components|GetUI)))))

(event Game|Damage|EventAnyDamage
  (params (Damage :type Float%20%28single-precision%29) (DamageType :type Damage%20Type%20Object%20Reference) (InstigatedBy :type Controller%20Object%20Reference) (DamageCauser :type Actor%20Object%20Reference))
  ;[0.15 0.15 0.15 0.5] Damage
  (Class|BPIUI|SetHealthBar(Message) (Variables|Components|GetUI) Damage)
  (bind _output_get (Variables|Default|SetHealth (- (Variables|Default|GetHealth) Damage)))
  (if (<= _output_get 0.0)
    (CallFunction|Die)))

(event EventSetInputEnabled
  (params (Enabled :type Boolean))
  ;[0.15 0.15 0.15 0.5] Input Toggle
  (if Enabled
    (Input|EnableInput 0)
    (else
      (Input|DisableInput 0))))

(event EventBeginPlay
  ;[0.15 0.15 0.15 0.5] Init
  (Utilities|FlowControl|Sequence
    (:then_0
      (bind _returnvalue (UserInterface|CreateWidget "/Game/UI/Player/WB_HUD.WB_HUD_C"))
      (bind _output_get (Variables|Components|SetUI _returnvalue))
      (UserInterface|Viewport|AddtoViewport _output_get 0))
    (:then_1
      (Variables|/Script/Engine.CharacterMovementComponent|SetMaxWalkSpeed (Variables|Character|GetCharacterMovement) (Variables|Movement|GetwalkSpeed)))
    (:then_2
      (CallFunction|WeaponSwap)
      (CallFunction|AmmoUpdate (Variables|Default|GetCurrentAmmo)))))

(fn ConstructionScript
  (Utilities|FlowControl|Sequence
    (:then_0
      (Variables|Camera|SetbaseFov (Variables|/Script/Engine.CameraComponent|GetFieldOfView (Variables|Default|GetCamera))))
    (:then_1
      (Variables|Default|SetCurrentAmmo (Variables|Default|GetstartingAmmo)))))

(fn RocketReloadNotify
  (params (Selection :type Name))
  (switch name Selection
    (:reloaded
      (Variables|Default|SetcanReload? false))
    (:Reloading
      (if (not (> (Variables|Default|GetCurrentAmmo) 0))
        (Class|AnimInstance|StopSlotAnimation (Components|SkeletalMesh|GetAnimInstance (Variables|Default|GetArmRig)) 0.25 "None")))
    (:armLowered
      (Components|SkinnedMesh|UnHideBonebyName (Variables|Default|GetWeapon) "Rocket1")
      (Variables|Default|SetcanShoot true)
      (CallFunction|AmmoUpdate (Variables|Default|GetCurrentAmmo)))))

(fn LureTrace
  (bind _camera (Variables|Default|GetCamera))
  (bind _returnvalue (Transformation|GetWorldLocation _camera))
  (bind (_outhit _returnvalue_2) (Collision|LineTraceByChannel _returnvalue (+ _returnvalue (* (Math|Vector|GetForwardVector _camera) (Variables|Default|GetLureRange))) "TraceTypeQuery2" false 0 "ForOneFrame"))
  (return (.HitActor (Collision|BreakHitResult _outhit)) (and _returnvalue_2 (Utilities|IsValid (.HitActor (Collision|BreakHitResult _outhit))))))

(fn AmmoUpdate
  (params (Ammo :type Integer))
  (bind _ui (Variables|Components|GetUI))
  (Class|BPIUI|UpdateLoadedAmmo(Message) _ui 1)
  (Class|BPIUI|UpdateReserveAmmo(Message) _ui (Math|Integer|Clamp(Integer) (- Ammo 1) 0 (Variables|Default|GetstartingAmmo))))

(fn CanbeDetected
  (bind _currentweapon (Variables|Default|GetcurrentWeapon))
  (Development|PrintString (Utilities|String|EnumtoString _currentweapon))
  (return (Utilities|Select :Index _currentweapon :NewEnumerator0 false :NewEnumerator1 true)))

(fn GetCamera
  (return (Variables|Default|GetCamera)))