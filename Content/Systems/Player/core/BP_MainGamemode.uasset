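; Main game mode that runs a target-killing level: score, police bounty, dynamic music and win/lose flow.
; CallPolice and accumulated AddBounty thresholds raise the bounty tier once each, granting score and multiplier boosts and broadcasting to the HUD.
; That broadcast drives MusicSwitch, which unmutes music loops all started together at BeginPlay.
; Target escape, Lose, or player exit with a dead target shows a result screen, fades and opens the main menu.
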(event Custom|OnTargetEscape
  ;[0.7656 0.279 0.6701 0.5] Target Events
  (Development|PrintString "TARGET ESCAPE YOU FAIL YOU FAIL" true true "(R=1.000000,G=0.061364,B=0.000000,A=1.000000)" 5.0)
  (bind _returnvalue (UserInterface|CreateWidget "/Game/UI/Player/WB_LoseScreen.WB_LoseScreen_C"))
  (UserInterface|Viewport|AddtoViewport _returnvalue 0)
  (Class|BPIPlayer|SetInputEnabled(Message) (Game|GetPlayerCharacter 0) false)
  (Utilities|FlowControl|Delay 2.0)
  (CallFunction|CreateFade 1.0)
  (Utilities|FlowControl|Delay 1.0)
  (Game|OpenLevel(byName) "MAINMENU"))

(event Custom|OnTargetDeath
  ;[0.7656 0.279 0.6701 0.5] Target Events
)

(event Custom|PrepMusic
  ;[0.15 0.15 0.15 0.5] Prepares and plays All audio tracks, Mutes unneeded tracks
  (Utilities|FlowControl|Sequence
    (:then_0
      (bind _returnvalue (Audio|CreateSound2D "/Game/Audio/MusicTracks/Calm/CalmLoop.CalmLoop" 1.0 1.0 0.0 0))
      (Variables|Default|SetCalmLoop _returnvalue)
      (bind _returnvalue_2 (Audio|CreateSound2D "/Game/Audio/MusicTracks/Panic/PanicLoopBase.PanicLoopBase" 1.0 1.0 0.0 0))
      (Variables|Default|SetPanicLoopBase _returnvalue_2)
      (bind _returnvalue_3 (Audio|CreateSound2D "/Game/Audio/MusicTracks/Panic/PanicLoopMid.PanicLoopMid" 1.0 1.0 0.0 0))
      (Variables|Default|SetPanicLoopMid _returnvalue_3)
      (bind _returnvalue_4 (Audio|CreateSound2D "/Game/Audio/MusicTracks/Panic/PanicLoopMaxed.PanicLoopMaxed" 1.0 1.0 0.0 0))
      (Variables|Default|SetPanicLoopMax _returnvalue_4))
    (:then_1
      (Audio|Components|Audio|SetVolumeMultiplier (Variables|Default|GetCalmLoop) 0.25 :!class /Script/Engine.AudioComponent)
      (Audio|Components|Audio|Play (Variables|Default|GetCalmLoop) 0.0))
    (:then_2
      (Audio|Components|Audio|SetVolumeMultiplier (Variables|Default|GetPanicLoopBase) 0.0 :!class /Script/Engine.AudioComponent)
      (Audio|Components|Audio|Play (Variables|Default|GetPanicLoopBase) 0.0))
    (:then_3
      (Audio|Components|Audio|SetVolumeMultiplier (Variables|Default|GetPanicLoopMid) 0.0 :!class /Script/Engine.AudioComponent)
      (Audio|Components|Audio|Play (Variables|Default|GetPanicLoopMid) 0.0))
    (:then_4
      (Audio|Components|Audio|SetVolumeMultiplier (Variables|Default|GetPanicLoopMax) 0.0 :!class /Script/Engine.AudioComponent)
      (Audio|Components|Audio|Play (Variables|Default|GetPanicLoopMax) 0.0))))

(event Custom|MusicSwitch
  (params (BountyState :type E_Bounty%20Enum :default "NewEnumerator0"))
  ;[0.15 0.15 0.15 0.5] Dynamic Music
  (switch Utilities|FlowControl|Switch|SwitchonE_Bounty BountyState
    (:NewEnumerator1
      (Audio|Components|Audio|SetVolumeMultiplier (Variables|Default|GetCalmLoop) 0.0 :!class /Script/Engine.AudioComponent)
      (Audio|Components|Audio|SetVolumeMultiplier (Variables|Default|GetPanicLoopBase) 0.25 :!class /Script/Engine.AudioComponent))
    (:NewEnumerator2
      (Audio|Components|Audio|SetVolumeMultiplier (Variables|Default|GetPanicLoopMid) 0.25 :!class /Script/Engine.AudioComponent))
    (:NewEnumerator3
      (Audio|Components|Audio|SetVolumeMultiplier (Variables|Default|GetPanicLoopMax) 0.25 :!class /Script/Engine.AudioComponent))))

(event EventBeginPlay
  (Development|PrintString "GAME START" true true "(R=1.000000,G=0.000000,B=0.946029,A=1.000000)")
  ;[0.15 0.15 0.15 0.5] Dynamic Music
  (CallFunction|PrepMusic)
  (EventDispatchers|BindEventtoPlayerHudBountyUpdate (delegate Custom|MusicSwitch)))

(event EventTick
  (params (DeltaSeconds :type Float%20%28single-precision%29)))

(event EventApplyModifier
  (params (Modifier :type Float%20%28double-precision%29) (HudText :type String))
  ;[0.15 0.15 0.15 0.5] Score Applyers
  (bind _output_get (Variables|Default|SetScoreMult (+ Modifier (Variables|Default|GetScoreMult))))
  (Default|CallPlayerHudScoreTextUpdate HudText true)
  (Default|CallPlayerHudScoreMultUpdate _output_get))

(event EventAddBounty
  (params (val :type Float%20%28double-precision%29))
  ;[0.15 0.15 0.15 0.5] Add Bounty
  (bind _output_get (Variables|Default|SetbountyThreshold (+ (Variables|Default|GetbountyThreshold) val)))
  (if (and (>= _output_get 3.5e+02) (not (>= _output_get 7.5e+02)))
    (Utilities|FlowControl|DoOnce false
      (:Completed
        (bind _output_get_2 (Variables|Default|SetBountyLevel "NewEnumerator2"))
        (Default|CallPlayerHudBountyUpdate _output_get_2)
        (CallFunction|AddScore 5e+02 "THEY WANT YOU GONE")
        (CallFunction|ApplyScoreModifier 2.0 "BOUNTY INCREASED!")))
    (elif (>= _output_get 7.5e+02)
      (Utilities|FlowControl|DoOnce false
        (:Completed
          (bind _output_get_3 (Variables|Default|SetBountyLevel "NewEnumerator3"))
          (Default|CallPlayerHudBountyUpdate _output_get_3)
          (CallFunction|AddScore 1.5e+03 "KILL THEM ALL")
          (CallFunction|ApplyScoreModifier 5.0 "BOUNTY MAXIMISED!!!!"))))))

(event EventSwitchedWeapon
  (params (Armed? :type Boolean))
  ;[0.9427 0.8726 0.2995 0.5] DETECTION COMP
  (Default|CallWeaponSwitched Armed?))

(event EventCallPolice
  ;[0.9427 0.8726 0.2995 0.5] DETECTION COMP
  (Default|CallPoliceCalled)
  (Utilities|FlowControl|DoOnce false
    (:Completed
      (bind _output_get (Variables|Default|SetBountyLevel "NewEnumerator1"))
      (Default|CallPlayerHudBountyUpdate _output_get)
      (CallFunction|AddScore 1.5e+03 "WANTED")
      (CallFunction|ApplyScoreModifier 0.25 "BOUNTY BEGUN"))))

(event EventSwitchTargetState
  (params (NewState :type E_TargetState%20Enum :default "NewEnumerator0"))
  ;[0.5172 0.8906 0.2041 0.5] Target State
  (bind _output_get (Variables|Default|SetTargetState NewState))
  (switch Utilities|FlowControl|Switch|SwitchonE_TargetState _output_get
    (:NewEnumerator2
      (CallFunction|OnTargetEscape))))

(event EventPlayerExited
  ;[0.2 0.8125 0.6502 0.5] Player Events
  (switch Utilities|FlowControl|Switch|SwitchonE_TargetState (Variables|Default|GetTargetState)
    (:NewEnumerator0
      (Development|PrintString "YOU HAVENT KILLED THE EX"))
    (:NewEnumerator1
      (Development|PrintString "YOU WIN RAHHHHH" true true "(R=0.035564,G=1.000000,B=0.000000,A=1.000000)" 5.0)
      (bind _returnvalue (UserInterface|CreateWidget "/Game/UI/Player/WB_WinScreen.WB_WinScreen_C"))
      (UserInterface|Viewport|AddtoViewport _returnvalue 0)
      (Class|BPIPlayer|SetInputEnabled(Message) (Game|GetPlayerCharacter 0) false)
      (Utilities|FlowControl|Delay 2.0)
      (CallFunction|CreateFade 1.0)
      (Utilities|FlowControl|Delay 1.0)
      (Game|OpenLevel(byName) "MAINMENU"))))

(event EventFadeScreen
  (params (Duration :type Float%20%28double-precision%29))
  ;[0.04566 0.15 0.106 0.5] FadeScreen
  (CallFunction|CreateFade Duration))

(event EventLose
  ;[0.7656 0.279 0.6701 0.5] Target Events
  (Development|PrintString "TARGET ESCAPE YOU FAIL YOU FAIL" true true "(R=1.000000,G=0.061364,B=0.000000,A=1.000000)" 5.0)
  (bind _returnvalue (UserInterface|CreateWidget "/Game/UI/Player/WB_LoseScreen.WB_LoseScreen_C"))
  (UserInterface|Viewport|AddtoViewport _returnvalue 0)
  (Class|BPIPlayer|SetInputEnabled(Message) (Game|GetPlayerCharacter 0) false)
  (Utilities|FlowControl|Delay 2.0)
  (CallFunction|CreateFade 1.0)
  (Utilities|FlowControl|Delay 1.0)
  (Game|OpenLevel(byName) "MAINMENU"))

(event EventAddScore
  (params (Addition :type Float%20%28double-precision%29) (HudText :type String))
  ;[0.15 0.15 0.15 0.5] Score Applyers
  (bind _output_get (Variables|Default|SetScore (+ (* Addition (Variables|Default|GetScoreMult)) (Variables|Default|GetScore))))
  (Default|CallPlayerHudScoreTextUpdate HudText false)
  (Default|CallPlayerHudScoreValUpdate _output_get))

(event EventSubtractScore
  (params (Deduction :type Float%20%28double-precision%29) (HudText :type String))
  ;[0.15 0.15 0.15 0.5] Score Applyers
  (bind _output_get (Variables|Default|SetScore (- (Variables|Default|GetScore) Deduction)))
  (Default|CallPlayerHudScoreTextUpdate HudText false)
  (Default|CallPlayerHudScoreValUpdate _output_get))

(fn ConstructionScript)

(fn CreateFade
  (params (Duration :type Float%20%28double-precision%29))
  (bind _returnvalue (UserInterface|CreateWidget "/Game/UI/Effects/WB_Fade.WB_Fade_C"))
  (bind _output_get (LocalVariables|SetFadeRef _returnvalue))
  (UserInterface|Viewport|AddtoViewport _output_get 0)
  (Default|PlayFade _output_get Duration false))

(fn GetBounty
  (return (Variables|Default|GetBountyLevel)))

(fn GetScore
  (return (Variables|Default|GetScore)))