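; BP_Jackhammer is a roaming jackhammer hazard that spins erratically with a rocket trail and knocks characters away on contact.
; It chains AI MoveTo calls to random navigable points, while Tick randomizes its RotatingMovement rate.
; Box overlaps launch characters away from its center, stronger at closer range, gated by a DoOnce that resets after a short retriggerable delay.
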(event OnComponentBeginOverlap(Box)
  (params (OverlappedComponent :type Primitive%20Component%20Object%20Reference) (OtherActor :type Actor%20Object%20Reference) (OtherComp :type Primitive%20Component%20Object%20Reference) (OtherBodyIndex :type Integer) (bFromSweep :type Boolean) (SweepResult :type Hit%20Result%20Structure%20%28by%20ref%29))
  (bind _returnvalue (Transformation|GetActorLocation OtherActor))
  (bind _returnvalue_2 (Transformation|GetActorLocation))
  ;[0.15 0.15 0.15 0.5] Character Launching (credit Micheal, tweaked by Max)
  (bind _ascharacter (Utilities|Casting|CastToCharacter OtherActor))
  (Utilities|FlowControl|DoOnce false :!label _label
    (:Completed
      (Character|LaunchCharacter _ascharacter (* (Math|Vector|Normalize (- _returnvalue _returnvalue_2)) (Math|Float|MapRangeClamped (Math|Vector|Distance(Vector) _returnvalue_2 _returnvalue) 0.0 5e+02 1.5e+03 5e+02)) false false)
      (Utilities|FlowControl|RetriggerableDelay 0.5)
      (goto _label Reset))))

(event Custom|random%20move
  ;[0.15 0.15 0.15 0.5] random moving- ts turing like if it were a meerkat
  (if (not (> (Math|Vector|VectorLength (Transformation|GetVelocity)) 0.0))
    (bind _randomlocation (Class|NavigationSystemV1|GetRandomLocationinNavigableRadius (Transformation|GetActorLocation) 5e+03 0 0))
    (AI|AIMoveTo self _randomlocation 0 5.0 false
      (:OnSuccess
        _)
      (:OnFail
        _))
    (CallFunction|RandomMove)))

(event EventBeginPlay
  ;[0.15 0.15 0.15 0.5] set the rotation so that it can spin right and start trail
  (Transformation|SetActorRotation "0.000000,-33.000000,47.000000")
  (CallFunction|RandomMove)
  (Niagara|SpawnSystemAttached "/Game/Art/Particles/Trail/NS_RocketTrail.NS_RocketTrail" (Variables|Default|Getjackhammer) "None" "0, 0, 0" "0, 0, 0" "KeepRelativeOffset" false))

(event Collision|EventActorBeginOverlap
  (params (OtherActor :type Actor%20Object%20Reference)))

(event EventTick
  (params (DeltaSeconds :type Float%20%28single-precision%29))
  (bind _returnvalue (Math|Random|RandomFloatinRange 0.0 3.6e+02))
  ;[0.15 0.15 0.15 0.5] make it spin- it spins bad while moving, maybe fix it later
  (Variables|/Script/Engine.RotatingMovementComponent|SetRotationRate (Variables|Default|GetRotatingMovement) (Math|Rotator|MakeRotator 0.0 _returnvalue _returnvalue)))

(fn ConstructionScript)