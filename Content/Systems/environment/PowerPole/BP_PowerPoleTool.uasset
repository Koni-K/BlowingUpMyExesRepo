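; BP_PowerPoleTool is a construction-script tool that strings cables from one power pole to a linked Target pole.
; It applies the chosen static mesh, then, if Target is valid, adds a CableComponent at each mesh socket.
; Each cable ends at the same-index socket on Target, converted into this mesh's local space, with fixed width, material and gravity scale.
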(event EventBeginPlay)

(event Collision|EventActorBeginOverlap
  (params (OtherActor :type Actor%20Object%20Reference)))

(event EventTick
  (params (DeltaSeconds :type Float%20%28single-precision%29)))

(fn ConstructionScript
  (bind _target (Variables|Default|GetTarget))
  (bind _staticmesh (Variables|BP_PowerPoleTool_C|GetStaticMesh _target))
  (Components|StaticMesh|SetStaticMesh (Variables|Default|GetStaticMesh) (Variables|Default|GetNewStaticMesh))
  (Utilities|IsValid (Variables|Default|GetTarget)
    (:Is%20Valid
      (for (_array_element _array_index) (Transformation|GetAllSocketNames (Variables|Default|GetStaticMesh))
        (bind _returnvalue (AddComponent|AddCableComponent false))
        (Variables|/Script/CableComponent.CableComponent|SetCableWidth _returnvalue 15.0)
        (Rendering|Material|SetMaterial _returnvalue 0 "/Game/Art/Material/NPC/MI_SniperNPC.MI_SniperNPC")
        (Variables|/Script/CableComponent.CableComponent|SetCableGravityScale _returnvalue 15.0)
        (Transformation|SetWorldLocation _returnvalue (Transformation|GetSocketLocation (Variables|Default|GetStaticMesh) _array_element) false false)
        (Variables|/Script/CableComponent.CableComponent|SetEndLocation _returnvalue (Math|Transform|InverseTransformLocation (Transformation|GetWorldTransform (Variables|Default|GetStaticMesh)) (Transformation|GetSocketLocation _staticmesh (Utilities|Array|Get(acopy) (Transformation|GetAllSocketNames _staticmesh) _array_index))))))))