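; BP_Exit is an exit actor that reports to the game mode when the target or player reaches it.
; On actor overlap it checks the other actor against BP_TARGET, then BP_Player, sending a target state switch or a player-exited message respectively.
; A TargetRef death event switches the target to a different state through the same game mode message.
; Each handler also prints a debug string.
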(event OnDeath(TargetRef)
  (Development|PrintString "HOLD THE DICK AND BALLS")
  (Class|BPIGame|SwitchTargetState(Message) (Game|GetGameMode) "NewEnumerator1"))

(event Custom|Target%20Touched
  (Development|PrintString "TARGET TOUCHED")
  (Class|BPIGame|SwitchTargetState(Message) (Game|GetGameMode) "NewEnumerator2"))

(event Custom|Player%20Touched
  (Development|PrintString "PLAYER TOUCHED")
  (Class|BPIGame|PlayerExited(Message) (Game|GetGameMode)))

(event Collision|EventActorBeginOverlap
  (params (OtherActor :type Actor%20Object%20Reference))
  ;[1 0.8163 0.1274 0.5] Exit Collision
  (Class|KismetSystemLibrary|IsObjectOfSoftClass OtherActor "/Game/Systems/NPC/NPC_Children/Target/BP_TARGET.BP_TARGET_C"
    (:True
      (CallFunction|TargetTouched))
    (:False
      (Class|KismetSystemLibrary|IsObjectOfSoftClass OtherActor "/Game/Systems/Player/BP_Player.BP_Player_C"
        (:True
          (CallFunction|PlayerTouched))))))

(fn ConstructionScript)