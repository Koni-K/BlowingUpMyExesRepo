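; NPC component that detects a suspicious player and escalates through alert to calling the police.
; Sight updates and weapon-switch events start looping timers that raise detection faster at close range or drain it when sight is lost.
; An on-screen indicator shows the meter; full detection or a heard explosion triggers a timed alert, with a delayed police call notifying the gamemode.
; ForcePanic skips that notification and jumps straight to the final state.
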(event Custom|CE_RevertDetection
  (bind _osi (Variables|OSI|GetOSI))
  ;[0 0.651 0.5736 0.5] Revert Detection
  (bind _output_get (Variables|Detection|SetcurrentDetection (Math|Float|Clamp(Float) (- (Variables|Detection|GetcurrentDetection) 1.0) 0.0 1e+02)))
  (Class|BPIUI|SetHealthBar(Message) (Variables|OSI|GetOSI) (* _output_get 0.01))
  (if (== (Variables|Detection|GetcurrentDetection) 0.0)
    (Utilities|FlowControl|Sequence
      (:then_0
        ;;[0.15 0.15 0.15 0.5] Remove On Screen Indicator
        (Utilities|IsValid _osi
          (:Is%20Valid
            (Widget|RemovefromParent _osi)
            (Variables|OSI|SetIndicatorCreated false))))
      (:then_1
        (Utilities|Time|ClearandInvalidateTimerbyHandle (Variables|Detection|GetloseDetectionTime)))
      (:then_2
        (bind _output_get_2 (Variables|Default|SetcurrentState "NewEnumerator0"))
        (Default|CallSetPlayerState _output_get_2)))))

(event Custom|CallCops
  ;[0.1433 0.776 0.000887 0.5] 4 - Call Police
  (Default|ChangeIcon (Variables|OSI|GetOSI) "NewEnumerator2")
  (bind _returnvalue (Utilities|Time|SetTimerbyEvent (delegate Custom|PoliceCalled) (Variables|Call|GetPoliceCallLength)))
  (Variables|Call|SetPoliceTimer _returnvalue))

(event Custom|Sight
  (params (Actor :type Actor%20Object%20Reference) (Stimulus :type AI%20Stimulus%20Structure) (OSI%20Location :type Primitive%20Component%20Object%20Reference))
  (bind _bsuccessfullysensed (Utilities|Struct|BreakAIStimulus Stimulus))
  (bind _currentstate (Variables|Default|GetcurrentState))
  ;[0.8802 0 0.4299 0.5] 1 - On Sight Updated
  (Variables|Default|SetSuccessfully%20Sensed _bsuccessfullysensed)
  (if (or (Utilities|Enum|NotEqual(Enum) _currentstate "NewEnumerator2") (Utilities|Enum|NotEqual(Enum) _currentstate "NewEnumerator3"))
    (Utilities|FlowControl|Sequence
      (:then_0
        (Variables|OSI|SetOSI%20Location OSI%20Location))
      (:then_1
        (Class|KismetSystemLibrary|IsObjectOfSoftClass Actor "/Game/Systems/Player/BP_Player.BP_Player_C"
          (:True
            (Variables|Target|SetTarget Actor)
            (bind _output_get (Variables|Target|SetSensedPlayer? _bsuccessfullysensed))
            (bind _return (Class|BPIPlayer|CanbeDetected(Message) (Variables|Target|GetTarget)))
            (bind _output_get_2 (Variables|Target|SetcanDetect? _return))
            (if (and _output_get_2 _output_get)
              ;;[0 0.3181 1 0.5 12] GAINED SIGHT
              (CallFunction|CEGainedSight)
              (else
                ;;[1 0.3231 0 0.502 12] LOST SIGHT
                (CallFunction|CELostSight))))
          (:False
            ;;[0.15 0.15 0.15 0.5] Lost Sight of player
            (if (Variables|Target|GetSensedPlayer?)
              (Variables|Target|SetSensedPlayer? false)
              (Development|PrintString "LostSight"))))))))

(event Custom|CE_WeaponSwapCheck
  (params (Armed? :type Boolean))
  (bind _currentstate (Variables|Default|GetcurrentState))
  ;[0.4937 1 0.8263 0.5] Can detect if Armed
  (if (or (Utilities|Enum|Equal(Enum) _currentstate "NewEnumerator0") (Utilities|Enum|Equal(Enum) _currentstate "NewEnumerator1"))
    (bind _output_get (Variables|Target|SetcanDetect? Armed?))
    (Utilities|FlowControl|Sequence
      (:then_0
        (if (and _output_get (Variables|Target|GetSensedPlayer?))
          (CallFunction|CEGainedSight)
          (else
            (CallFunction|CELostSight)))))))

(event Custom|CE_Explosion%20heard
  (params (OSILOC :type Primitive%20Component%20Object%20Reference))
  ;[0.9153 1 0.001479 0.5] EXPLOSION HEARD
  (Variables|OSI|SetOSI%20Location OSILOC)
  (Utilities|FlowControl|Sequence
    (:then_0
      (CallFunction|ClearAllTimers))
    (:then_1
      (CallFunction|CreateOSI (Variables|OSI|GetOSI%20Location)))
    (:then_2
      ;;[1 0 0.1014 0.5] CE_Alert
      (CallFunction|CEAlert))))

(event Custom|PoliceCalled
  (bind _osi (Variables|OSI|GetOSI))
  ;[0.1433 0.776 0.000887 0.5] 4 - Call Police
  (Class|BPIGame|CallPolice(Message) (Game|GetGameMode))
  (bind _output_get (Variables|Default|SetcurrentState "NewEnumerator2"))
  (Default|CallSetPlayerState _output_get)
  (CallFunction|ClearAllTimers)
  (Utilities|IsValid _osi
    (:Is%20Valid
      (Widget|RemovefromParent _osi))))

(event Custom|CE_Detection
  ;[0.7031 0 0 0.5] 2 - Build Up Detection
  ;;[0.8 0.0487 0.1663 0.5] Rotate Towards Player
  (if (and (Utilities|Enum|Equal(Enum) (Variables|Default|GetcurrentState) "NewEnumerator1") (Variables|Target|GetcanDetect?))
    (if (Variables|Default|GetShouldRotatePlayer?)
      (Transformation|SetActorRotation (Variables|Default|Getowner) (Math|Rotator|MakeRotator 0.0 0.0 (.yaw (Math|Rotator|FindLookatRotation (Transformation|GetActorLocation (Variables|Default|Getowner)) (Transformation|GetActorLocation (Variables|Target|GetTarget)))))))
    ;;[0.8 0.0487 0.1663 0.5] Increase Detection - ( Closer - Higher, Further - Lower )
    (bind _output_get (Variables|Detection|SetcurrentDetection (Math|Float|Clamp(Float) (+ (Variables|Detection|GetcurrentDetection) (Math|Float|MapRangeClamped (Math|Vector|Distance(Vector) (Transformation|GetActorLocation (Variables|Default|Getowner)) (Transformation|GetActorLocation (Variables|Target|GetTarget))) 0.0 (Variables|Default|GetDetectionRange) (Variables|Detection|GetDetectionStrength) 0.0)) 0.0 1e+02)))
    (Class|BPIUI|SetHealthBar(Message) (Variables|OSI|GetOSI) (* _output_get 0.01))
    (if (== (* _output_get 0.01) 1.0)
      (CallFunction|CEAlert))
    (else
      (CallFunction|CELostSight))))

(event Custom|CE_Alert
  ;[1 0 0.1014 0.5] 3 - ALERT - NPC gets stunned for a duration of time then triggers the call police event
  (Utilities|Time|ClearandInvalidateTimerbyHandle (Variables|Detection|GetDetectionTime))
  (bind _output_get (Variables|Default|SetcurrentState "NewEnumerator3"))
  (Default|CallSetPlayerState _output_get)
  (Default|ChangeIcon (Variables|OSI|GetOSI) "NewEnumerator1")
  (bind _returnvalue (Utilities|Time|SetTimerbyEvent (EventDispatchers|CreateEvent :!event Custom|CallCops) (Variables|Alert|GetAlertLength)))
  (Variables|Alert|SetAlertTimer _returnvalue))

(event Custom|ForcePanic
  (bind _osi (Variables|OSI|GetOSI))
  ;[0.1433 0.776 0.000887 0.5] 4 - Call Police
  (bind _output_get (Variables|Default|SetcurrentState "NewEnumerator2"))
  (Default|CallSetPlayerState _output_get)
  (CallFunction|ClearAllTimers)
  (Utilities|IsValid _osi
    (:Is%20Valid
      (Widget|RemovefromParent _osi))))

(event Custom|CE_LostSight
  ;[1 0.3231 0 0.502] LOST SIGHT
  (Utilities|FlowControl|Sequence
    (:then_0
      (Utilities|Time|ClearandInvalidateTimerbyHandle (Variables|Detection|GetDetectionTime))
      (Development|PrintString "Lost Sight"))
    (:then_1
      (bind _returnvalue (Utilities|Time|SetTimerbyEvent (EventDispatchers|CreateEvent :!event Custom|CE_RevertDetection) 0.05 true))
      (Variables|Detection|SetloseDetectionTime _returnvalue))))

(event Custom|CE_GainedSight
  ;[0 0.3181 1 0.5] GAINED SIGHT
  (Utilities|FlowControl|Sequence
    (:then_0
      (if (Utilities|Time|IsValidTimerHandle (Variables|Detection|GetloseDetectionTime))
        (Utilities|Time|ClearandInvalidateTimerbyHandle (Variables|Detection|GetloseDetectionTime))))
    (:then_1
      (bind _output_get (Variables|Default|SetcurrentState "NewEnumerator1"))
      (Default|CallSetPlayerState _output_get)
      (Development|PrintString "Gained Sight"))
    (:then_2
      (if (not (Variables|OSI|GetIndicatorCreated))
        (CallFunction|CreateOSI (Variables|OSI|GetOSI%20Location))
        (Variables|OSI|SetIndicatorCreated true)))
    (:then_3
      (bind _returnvalue (Utilities|Time|SetTimerbyEvent (EventDispatchers|CreateEvent :!event Custom|CE_Detection) 0.05 true))
      (Variables|Detection|SetDetectionTime _returnvalue))))

(event EventEndPlay
  (params (EndPlayReason :type EEndPlayReason%20Enum :default "Destroyed"))
  (bind _osi (Variables|OSI|GetOSI))
  ;[0.15 0.01416 0.01129 0.5] EndPlay
  (Utilities|Time|ClearandInvalidateTimerbyHandle (Variables|Call|GetPoliceTimer))
  (Utilities|Time|ClearandInvalidateTimerbyHandle (Variables|Alert|GetAlertTimer))
  (Utilities|Time|ClearandInvalidateTimerbyHandle (Variables|Detection|GetloseDetectionTime))
  (Utilities|Time|ClearandInvalidateTimerbyHandle (Variables|Detection|GetDetectionTime))
  (Utilities|IsValid _osi
    (:Is%20Valid
      (Widget|RemovefromParent _osi))))

(event EventTick
  (params (DeltaSeconds :type Float%20%28single-precision%29)))

(event EventBeginPlay
  ;[0.15 0.15 0.15 0.5] Init
  (Variables|Default|Setowner (Components|GetOwner))
  (bind _asbp_main_gamemode (Utilities|Casting|CastToBP_MainGamemode (Game|GetGameMode)))
  (Variables|Default|SetAs%20BP%20Main%20Gamemode _asbp_main_gamemode)
  (Utilities|FlowControl|Sequence
    (:then_0
      (EventDispatchers|BindEventtoPoliceCalled (Variables|Default|GetAs%20BP%20Main%20Gamemode) (EventDispatchers|CreateEvent :!event Custom|ForcePanic)))
    (:then_1
      (EventDispatchers|BindEventtoWeaponSwitched (Variables|Default|GetAs%20BP%20Main%20Gamemode) (EventDispatchers|CreateEvent :!event Custom|CE_WeaponSwapCheck)))))

(fn CreateOSI
  (params (targetedComponent :type Primitive%20Component%20Object%20Reference))
  (Utilities|IsValid (Variables|OSI|GetOSI)
    (:Is%20Valid
      (Widget|RemovefromParent (Variables|OSI|GetOSI)))
    (:Is%20Not%20Valid
      _))
  (bind _returnvalue (UserInterface|CreateWidget "/Game/UI/Physical/OSI/WB_OSI.WB_OSI_C" 0 targetedComponent))
  (bind _output_get (Variables|OSI|SetOSI _returnvalue))
  (UserInterface|Viewport|AddtoViewport _output_get 0))

(fn ClearAllTimers
  (bind _detectiontime (Variables|Detection|GetDetectionTime))
  (bind _losedetectiontime (Variables|Detection|GetloseDetectionTime))
  (bind _alerttimer (Variables|Alert|GetAlertTimer))
  (Utilities|FlowControl|Sequence
    (:then_0
      (if (Utilities|Time|IsValidTimerHandle _losedetectiontime)
        (Utilities|Time|ClearandInvalidateTimerbyHandle _losedetectiontime)))
    (:then_1
      (if (Utilities|Time|IsValidTimerHandle _detectiontime)
        (Utilities|Time|ClearandInvalidateTimerbyHandle _detectiontime)))
    (:then_2
      (if (Utilities|Time|IsValidTimerHandle _alerttimer)
        (Utilities|Time|ClearandInvalidateTimerbyHandle _alerttimer)))))