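; BP_Civ is a civilian NPC that detects the player through AI perception and escalates to a police call.
; While sensed, a looping timer turns it toward the player and fills a detection meter scaled by distance, shown on a WB_OSI on-screen indicator.
; Losing sight drains the meter back to the initial state.
; A full meter locks the alert state and starts a delayed CallCops, which currently only swaps the icon and prints.
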(event OnTargetPerceptionUpdated(AIPerception)
  (params (Actor :type Actor%20Object%20Reference) (Stimulus :type AI%20Stimulus%20Structure))
  (if (Utilities|Enum|NotEqual(Enum) (Variables|Default|GetcurrentState) "NewEnumerator2")
    (Class|KismetSystemLibrary|IsObjectOfSoftClass Actor "/Game/Systems/Player/BP_Player.BP_Player_C"
      (:True
        (Variables|Default|SetTarget Actor)
        (if (.bSuccessfullySensed (Utilities|Struct|BreakAIStimulus Stimulus))
          (if (Utilities|Time|IsValidTimerHandle (Variables|Default|GetloseDetectionTime))
            (Utilities|Time|ClearandInvalidateTimerbyHandle (Variables|Default|GetloseDetectionTime)))
          (Utilities|FlowControl|Sequence
            (:then_0
              (Variables|Default|SetcurrentState "NewEnumerator1"))
            (:then_1
              (Utilities|IsValid (Variables|Default|GetOSI)
                (:Is%20Valid
                  (Widget|RemovefromParent (Variables|Default|GetOSI)))
                (:Is%20Not%20Valid
                  _))
              (bind _returnvalue (UserInterface|CreateWidget "/Game/UI/Physical/OSI/WB_OSI.WB_OSI_C" 0 (Variables|Default|GetSphere1)))
              (bind _output_get (Variables|Default|SetOSI _returnvalue))
              (UserInterface|Viewport|AddtoViewport _output_get 0)
              (Development|PrintString "Detection"))
            (:then_2
              (bind _returnvalue_2 (Utilities|Time|SetTimerbyEvent (delegate Custom|Detection) 0.01 true))
              (Variables|Default|SetDetectionTime _returnvalue_2)))
          (else
            (Utilities|FlowControl|Sequence
              (:then_0
                (Development|PrintString "Lost Sight"))
              (:then_1
                (Utilities|Time|ClearandInvalidateTimerbyHandle (Variables|Default|GetDetectionTime)))
              (:then_2
                (bind _returnvalue_3 (Utilities|Time|SetTimerbyEvent (delegate Custom|RevertDetection) 0.1 true))
                (Variables|Default|SetloseDetectionTime _returnvalue_3)))))))))

(event Custom|RevertDetection
  (bind _osi (Variables|Default|GetOSI))
  (bind _output_get (Variables|Default|SetcurrentDetection (Math|Float|Clamp(Float) (- (Variables|Default|GetcurrentDetection) 2.5) 0.0 1e+02)))
  (Class|BPIUI|SetHealthBar(Message) (Variables|Default|GetOSI) (* _output_get 0.01))
  (Development|PrintString (Utilities|String|ToString(Float) (Math|Float|Clamp(Float) (- (Variables|Default|GetcurrentDetection) 2.5) 0.0 1e+02)))
  (if (== _output_get 0.0)
    (Utilities|FlowControl|Sequence
      (:then_0
        ;[0.15 0.15 0.15 0.5] Remove On Screen Indicator
        (Utilities|IsValid _osi
          (:Is%20Valid
            (Widget|RemovefromParent _osi))))
      (:then_1
        (Utilities|Time|ClearandInvalidateTimerbyHandle (Variables|Default|GetloseDetectionTime)))
      (:then_2
        (Variables|Default|SetcurrentState "NewEnumerator0")))))

(event Custom|CallCops
  (Default|ChangeIcon (Variables|Default|GetOSI) "NewEnumerator2")
  (Development|PrintString "Police"))

(event Custom|Detection
  (Transformation|SetActorRotation (Math|Rotator|MakeRotator 0.0 0.0 (.yaw (Math|Rotator|FindLookatRotation (Transformation|GetActorLocation) (Transformation|GetActorLocation (Variables|Default|GetTarget))))))
  (bind _output_get (Variables|Default|SetcurrentDetection (Math|Float|Clamp(Float) (+ (Variables|Default|GetcurrentDetection) (Math|Float|MapRangeClamped (Math|Vector|Distance(Vector) (Transformation|GetActorLocation) (Transformation|GetActorLocation (Variables|Default|GetTarget))) 0.0 3e+03 (Variables|Default|GetDetectionStrength) 0.0)) 0.0 1e+02)))
  (Class|BPIUI|SetHealthBar(Message) (Variables|Default|GetOSI) (* _output_get 0.01))
  (if (== (* _output_get 0.01) 1.0)
    (Utilities|Time|ClearandInvalidateTimerbyHandle (Variables|Default|GetDetectionTime))
    (Variables|Default|SetcurrentState "NewEnumerator2")
    (Default|ChangeIcon (Variables|Default|GetOSI) "NewEnumerator1")
    (bind _returnvalue (Utilities|Time|SetTimerbyEvent (delegate Custom|CallCops) (Variables|Default|GetAlertLength)))
    (Variables|Default|SetAlertTimer _returnvalue)
    (Development|PrintString (Utilities|String|ToString(Float) (Utilities|Time|GetTimerRemainingTimebyHandle _returnvalue)))))

(event EventAlert
  (params (Instigator :type Actor%20Object%20Reference)))

(fn ConstructionScript)