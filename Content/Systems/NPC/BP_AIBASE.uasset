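; Base NPC AI that wanders, reacts to players and explosions, and can be lured or killed.
; A CurrentState switch in Decide drives behavior, looping after moves, with Detecting, AlertState and CanLure left as stubs.
; BPCDetection receives player sightings and the first heard explosion, which turns the NPC toward its instigator.
; Panic, preset when game-mode stealth is broken, wanders at panic speed and flees rocket blasts via an opposite-direction offset.
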(event OnTargetPerceptionUpdated(AIPerception)
  (params (Actor :type Actor%20Object%20Reference) (Stimulus :type AI%20Stimulus%20Structure))
  ;[0.1755 0.9948 0.00235 0.5] Detection
  (if (Actor|ActorHasTag Actor "Player")
    (Default|Sight (Variables|Default|GetBPC_Detection) Actor Stimulus (Variables|Default|GetSphere1))))

(event Custom|Decide
  ;[0.000687 0.4304 0.6198 0.5] Deciding State
  (switch Utilities|FlowControl|Switch|SwitchonE_State (Variables|Default|GetcurrentState)
    (:NewEnumerator0
      (CallFunction|NormalState))
    (:NewEnumerator1
      (Class|NavMovementInterface|StopActiveMovement (Variables|Character|GetCharacterMovement))
      (CallFunction|Detecting))
    (:NewEnumerator3
      (CallFunction|AlertState))
    (:NewEnumerator2
      (CallFunction|PanicState)
      (Variables|/Script/Engine.CharacterMovementComponent|SetMaxWalkSpeed (Variables|Character|GetCharacterMovement) (Variables|Default|GetpanicWalkSpeed)))))

(event Custom|Detecting)

(event Custom|SetState
  (params (State :type E_State%20Enum :default "NewEnumerator0"))
  ;[0.000687 0.4304 0.6198 0.5] Deciding State
  (Variables|Default|SetcurrentState State)
  (switch Utilities|FlowControl|Switch|SwitchonE_State (Variables|Default|GetcurrentState)
    (:NewEnumerator0
      (CallFunction|NormalState))
    (:NewEnumerator1
      (Class|NavMovementInterface|StopActiveMovement (Variables|Character|GetCharacterMovement))
      (CallFunction|Detecting))
    (:NewEnumerator3
      (CallFunction|AlertState))
    (:NewEnumerator2
      (CallFunction|PanicState)
      (Variables|/Script/Engine.CharacterMovementComponent|SetMaxWalkSpeed (Variables|Character|GetCharacterMovement) (Variables|Default|GetpanicWalkSpeed)))))

(event Custom|Panic%20State
  (bind _returnvalue (Transformation|GetActorLocation))
  ;[0 0.9167 0.09948 0.5] Panic Wander
  (bind (_randomlocation _returnvalue_2) (Class|NavigationSystemV1|GetRandomLocationinNavigableRadius (select (Variables|Default|GetrunFromRocket?) (+ _returnvalue (* (* (Math|Vector|Normalize (- (Variables|Default|GetRocketLoc) _returnvalue)) -1.0) 1e+03)) (Transformation|GetActorLocation)) 1.5e+03 0 0))
  (if _returnvalue_2
    (AI|AIMoveTo self _randomlocation 0 5.0 false
      (:OnSuccess
        (Development|PrintString "SUCCESS"))
      (:OnFail
        (Development|PrintString "FAIL")))
    (Variables|Default|SetrunFromRocket? false)
    (CallFunction|Decide)))

(event Custom|NormalState
  ;[0.295 0.1367 0.9479 0.5] Regular Wander Logic
  (if (not (> (Math|Vector|VectorLength (Transformation|GetVelocity)) 0.0))
    (bind _randomlocation (Class|NavigationSystemV1|GetRandomLocationinNavigableRadius (Transformation|GetActorLocation) (Variables|Default|GetWalkRadius) 0 0))
    (AI|AIMoveTo self _randomlocation 0 5.0 false
      (:OnSuccess
        _)
      (:OnFail
        _))
    (CallFunction|Decide)))

(event Custom|AlertState)

(event EventBeginPlay
  (Utilities|FlowControl|Sequence
    (:then_0
      (bind _asbp_main_gamemode (Utilities|Casting|CastToBP_MainGamemode (Game|GetGameMode)))
      (if (Variables|/Game/Systems/Player/core/BP_MainGamemode.BP_MainGamemode_C|GetStealthBroken? _asbp_main_gamemode)
        (Variables|Default|SetcurrentState "NewEnumerator2")))
    (:then_1
      (EventDispatchers|BindEventtoSetPlayerState (Variables|Default|GetBPC_Detection) (EventDispatchers|CreateEvent :!event Custom|SetState))
      (Variables|/Script/Engine.CharacterMovementComponent|SetMaxWalkSpeed (Variables|Character|GetCharacterMovement) (Variables|Default|GetnormalWalkSpeed))
      (Utilities|FlowControl|Delay 3.0)
      (CallFunction|Decide))))

(event EventAlert
  (params (Instigator :type Actor%20Object%20Reference) (RocketLocation :type Vector :default "0, 0, 0"))
  ;[0.7188 0 0.6967 0.5] Alerted by Nearby Explosion
  (Variables|Default|SetRocketLoc RocketLocation)
  (switch Utilities|FlowControl|Switch|SwitchonE_State (Variables|Default|GetcurrentState)
    (:NewEnumerator0
      (Utilities|FlowControl|DoOnce false :!label _label
        (:Completed
          (Transformation|SetActorRotation (Math|Rotator|MakeRotator 0.0 0.0 (.yaw (Math|Rotator|FindLookatRotation (Transformation|GetActorLocation) (Transformation|GetActorLocation Instigator)))))
          (Default|CEExplosionHeard (Variables|Default|GetBPC_Detection) (Variables|Default|GetSphere1))
          (Variables|Default|SetcurrentState "NewEnumerator1")
          (CallFunction|Decide))))
    (:NewEnumerator1
      (goto _label))
    (:NewEnumerator2
      (Class|NavMovementInterface|StopActiveMovement (Variables|Character|GetCharacterMovement))
      (Variables|Default|SetrunFromRocket? true)
      (CallFunction|PanicState))))

(event EventKill
  (params (Instigator :type Actor%20Object%20Reference))
  (Game|SpawnActorfromClass "/Game/Systems/Particle/BP_ParticleActor.BP_ParticleActor_C" (Transformation|GetActorTransform) "Undefined" "MultiplyWithRoot" 0 "/Game/Art/Particles/ConfetiKill/NS_KILL.NS_KILL" 0)
  (Actor|DestroyActor))

(event EventLure
  (params (ActorToFollow :type Actor%20Object%20Reference))
  ;[0.15 0.15 0.15 0.5] Lure
  (Game|SpawnActorfromClass "/Game/Systems/Particle/BP_ParticleActor.BP_ParticleActor_C" (Transformation|GetActorTransform) "Undefined" "MultiplyWithRoot" 0 "/Game/Art/Particles/Enamored/NS_Enamored.NS_Enamored" 0)
  (AI|AIMoveTo self "0, 0, 0" ActorToFollow 5.0 false
    (:OnSuccess
      _)
    (:OnFail
      _))
  (CallFunction|Decide))

(fn ConstructionScript)

(fn CanLure?
  (return false))