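; Civilian NPC child Blueprint that sets the score consequences of killing a civilian.
; Its Kill override switches on the bounty tier: lower tiers deduct score with a regret message, Dead or Alive also increases bounty, and Threat to Society awards a bloodlust bonus.
; It then runs the parent Kill logic.
; CanLure returns true only while the NPC is in one specific state.
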(event EventBeginPlay
  (|CallParentFunction) ; This node is disabled and will not be called.\nDrag off pins to build functionality.
)

(event Collision|EventActorBeginOverlap
  (params (OtherActor :type Actor%20Object%20Reference)))

(event EventTick
  (params (DeltaSeconds :type Float%20%28single-precision%29)))

(event EventKill
  (params (Instigator :type Actor%20Object%20Reference))
  (Utilities|FlowControl|Sequence
    (:then_0
      (bind _e_bounty (CallFunction|GetBounty))
      (switch Utilities|FlowControl|Switch|SwitchonE_Bounty _e_bounty
        (:NewEnumerator0
          (CallFunction|RemoveScore 5e+01 "OOPS I SHOULDNT HAVE DONE THAT" :!label _label))
        (:NewEnumerator1
          (Utilities|FlowControl|Sequence
            (:then_0
              (goto _label))))
        (:NewEnumerator2
          (Utilities|FlowControl|Sequence
            (:then_0
              (goto _label))
            (:then_1
              (CallFunction|IncreaseBounty 1e+02))))
        (:NewEnumerator3
          (CallFunction|AddScore 2.5e+02 "BLOODLUST"))))
    (:then_1
      (|CallParentFunction Instigator))))

(fn ConstructionScript
  (|CallParentFunction))

(fn CanLure?
  (return (Utilities|Enum|Equal(Enum) (Variables|Default|GetcurrentState) "NewEnumerator0")))