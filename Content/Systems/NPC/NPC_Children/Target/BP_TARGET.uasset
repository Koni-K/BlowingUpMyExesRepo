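; Target NPC child Blueprint that overrides the panic, lure and death behavior of its parent.
; Panic loops AI moves to random navigable points, offset away from the rocket when flagged, until sprinting is enabled, and starts a one-time timer.
; Escape raises walk speed and heads for a random exit, retrying on failure.
; Luring is allowed only in the normal state and fires detection's explosion-heard event once; death calls OnDeath before parent logic.
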(event Custom|Escape%20State
  ;[0.7292 0.04618 0.04374 0.5] Run State
  (Variables|Default|SetCanSprint true)
  (Development|PrintString "RUN MI AMIGOS")
  (Variables|/Script/Engine.CharacterMovementComponent|SetMaxWalkSpeed (Variables|Character|GetCharacterMovement) 1e+03)
  (Utilities|FlowControl|RetriggerableDelay 0.2 :!label _label)
  (AI|AIMoveTo self (Transformation|GetActorLocation (.OutItem (Utilities|Array|Random (Variables|Default|GetExits)))) 0 5.0 false
    (:OnFail
      (goto _label))))

(event EventBeginPlay
  (|CallParentFunction) ; This node is disabled and will not be called.\nDrag off pins to build functionality.
)

(event Collision|EventActorBeginOverlap
  (params (OtherActor :type Actor%20Object%20Reference)))

(event EventTick
  (params (DeltaSeconds :type Float%20%28single-precision%29)))

(event EventPanicState
  ;[0.9323 0.4762 0.147 0.5] Custom Target Class Panic Override
  (Utilities|FlowControl|Sequence
    (:then_0
      (bind _location (CallFunction|RandomLocationinRange 1.5e+03 :!label _label))
      (AI|AIMoveTo self _location 0 5.0 false
        (:OnSuccess
          _)
        (:OnFail
          _))
      (if (not (Variables|Default|GetCanSprint))
        (goto _label)))
    (:then_1
      (Utilities|FlowControl|DoOnce false
        (:Completed
          (Utilities|Time|SetTimerbyEvent (EventDispatchers|CreateEvent :!event Custom|Escape%20State) 1e+01))))))

(event EventKill
  (params (Instigator :type Actor%20Object%20Reference))
  ;[0.8281 0 0.6803 0.5] Death Override
  (Default|CallOnDeath)
  (|CallParentFunction 0))

(event EventLure
  (params (ActorToFollow :type Actor%20Object%20Reference))
  ;[0.3553 0.9375 0.7357 0.5] Lure Override
  (Utilities|FlowControl|DoOnce false
    (:Completed
      (Development|PrintString "ITS YOU!!!")
      (Default|CEExplosionHeard (Variables|Default|GetBPC_Detection) (Variables|Default|GetSphere1)))))

(fn ConstructionScript
  (|CallParentFunction))

(fn RandomLocationinRange
  (params (Range :type Float%20%28double-precision%29))
  (bind _returnvalue (Transformation|GetActorLocation))
  (bind (_randomlocation _returnvalue_2) (Class|NavigationSystemV1|GetRandomLocationinNavigableRadius (select (Variables|Default|GetrunFromRocket?) (+ _returnvalue (* (* (Math|Vector|Normalize (- (Variables|Default|GetRocketLoc) _returnvalue)) -1.0) 1e+03)) "0, 0, 0") Range 0 0))
  (return _returnvalue_2 _randomlocation))

(fn CanLure?
  (return (Utilities|Select :Index (Variables|Default|GetcurrentState) :NewEnumerator0 true :NewEnumerator1 false :NewEnumerator3 false :NewEnumerator2 false)))