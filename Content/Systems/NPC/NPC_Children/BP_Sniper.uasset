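; Sniper NPC child that watches for the player with a sweeping vision cone and a visible laser.
; In Normal state it plays sweep timelines and runs a looping timer that tests a dot-product cone plus line trace, reporting the player to BPCDetection.
; Tick aims the laser along the offset forward vector in Normal, lerps it toward the player in Detecting and Panic, and scales its length by trace distance.
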(event Custom|NormalVisionSweep
  ;[0.15 0.15 0.15 0.5] Normal State
  (bind (_playerblocked _dottrue_) (CallFunction|SweepingConeVision))
  (if _dottrue_
    (Utilities|Time|ClearandInvalidateTimerbyHandle (Variables|Default|GetnormalVisionSweepTimer))
    (if _playerblocked
      (Default|Sight (Variables|Default|GetBPC_Detection) (Variables|Default|Getplayer) (Utilities|Struct|MakeAIStimulus 0.0 0.0) (Variables|Default|GetSphere1))
      (Development|PrintString "SNIPERSIGHT")
      (CallFunction|Decide)
      (else
        (Default|Sight (Variables|Default|GetBPC_Detection) (Variables|Default|Getplayer) (Utilities|Struct|MakeAIStimulus 0.0 0.0 -1.0 "340282346638528859811704183484516925440.000000,340282346638528859811704183484516925440.000000,340282346638528859811704183484516925440.000000" "340282346638528859811704183484516925440.000000,340282346638528859811704183484516925440.000000,340282346638528859811704183484516925440.000000" "None" true) (Variables|Default|GetSphere1))
        (Development|PrintString "SNIPERSIGHT SIGHT")))))

(event EventBeginPlay
  ;[0.15 0.15 0.15 0.5] Init
  (Utilities|FlowControl|Sequence
    (:then_0
      (bind _returnvalue (Actor|GetActorOfClass "/Game/Systems/Player/BP_Player.BP_Player_C"))
      (Utilities|IsValid _returnvalue
        (:Is%20Valid
          (Variables|Default|Setplayer _returnvalue))))
    (:then_1
      (|CallParentFunction))))

(event Collision|EventActorBeginOverlap
  (params (OtherActor :type Actor%20Object%20Reference)))

(event EventTick
  (params (DeltaSeconds :type Float%20%28single-precision%29))
  (bind _currentstate (Variables|Default|GetcurrentState))
  (bind _laser (Variables|Default|Getlaser))
  (bind _laser_2 (Variables|Default|Getlaser))
  (bind _returnvalue (Transformation|GetWorldLocation _laser_2))
  (Utilities|FlowControl|Sequence
    (:then_0
      (Development|PrintString (Utilities|String|EnumtoString _currentstate)))
    (:then_2
      (switch Utilities|FlowControl|Switch|SwitchonE_State _currentstate
        (:NewEnumerator0
          ;[0.15 0.15 0.15 0.5] Normal Length Trace
          (bind _laserotation (CallFunction|LaserLengthTrace (Transformation|GetWorldLocation (Variables|Default|Getlaser)) (* (+ (Transformation|GetActorForwardVector) (Math|Transform|InverseTransformDirection (Transformation|GetActorTransform) (Variables|Default|GetOffset))) 1.5e+04)))
          (Transformation|SetWorldRotation (Variables|Default|Getlaser) _laserotation false false))
        (:NewEnumerator1
          (Transformation|SetWorldRotation (Variables|Default|Getlaser) (Math|Rotator|Lerp(Rotator) (Transformation|GetWorldRotation _laser) (Math|Rotator|FindLookatRotation (Transformation|GetWorldLocation _laser) (Transformation|GetActorLocation (Variables|Default|Getplayer))) (* (Utilities|Time|GetWorldDeltaSeconds) (Variables|Default|GetCorrection%20Speed))) false false :!label _label)
          (CallFunction|LaserLengthTrace _returnvalue (+ _returnvalue (* (Math|Vector|GetForwardVector _laser_2) 1.5e+04))))
        (:NewEnumerator2
          (goto _label))))))

(event EventNormalState
  (bind _detectingvisionsweeptimer (Variables|Default|GetDetectingVisionSweepTimer))
  ;[0.15 0.15 0.15 0.5] Normal State
  (if (Utilities|Time|IsValidTimerHandle _detectingvisionsweeptimer)
    (Utilities|FlowControl|Sequence
      (:then_0
        (Audio|Components|Audio|Play (Variables|Default|GetHorizontalSweep))
        (Audio|Components|Audio|Play (Variables|Default|GetVerticalSweep)))
      (:then_1
        (Utilities|Time|ClearandInvalidateTimerbyHandle _detectingvisionsweeptimer)
        (if (Utilities|Time|IsValidTimerHandle (Variables|Default|GetnormalVisionSweepTimer)) :!label _label
          (Utilities|Time|ClearandInvalidateTimerbyHandle (Variables|Default|GetnormalVisionSweepTimer)))
        (bind _returnvalue (Utilities|Time|SetTimerbyEvent (delegate Custom|NormalVisionSweep) 0.1 true))
        (Variables|Default|SetnormalVisionSweepTimer _returnvalue)))
    (else
      (goto _label))))

(event EventDetecting
  (Utilities|FlowControl|Sequence
    (:then_0
      (Audio|Components|Audio|Stop (Variables|Default|GetVerticalSweep))
      (Audio|Components|Audio|Stop (Variables|Default|GetHorizontalSweep))
      (Utilities|Time|ClearandInvalidateTimerbyHandle (Variables|Default|GetnormalVisionSweepTimer)))
    (:then_1
      (bind _returnvalue (Utilities|Time|SetTimerbyEvent 0 0.01 true))
      (Variables|Default|SetDetectingVisionSweepTimer _returnvalue)
      (Variables|Default|SetStartRot (Transformation|GetWorldRotation (Variables|Default|Getlaser))))))

(event EventPanicState
  (Variables|Default|SetStartRot (Transformation|GetWorldRotation (Variables|Default|Getlaser))))

(fn ConstructionScript
  (|CallParentFunction)
  (Variables|Default|Setvision (Math|Trig|Cos(Degrees) (Variables|Default|GetFieldOfView))))

(fn SweepingConeVision
  (bind _player (Variables|Default|Getplayer))
  ;[0.5469 0.2822 0 0.5] Custom Cone Vision Check
  (Variables|Default|SetFacingVec (Math|Vector|Normalize (+ (Transformation|GetActorForwardVector) (Math|Transform|InverseTransformDirection (Transformation|GetActorTransform) (Variables|Default|GetOffset)))))
  (Utilities|IsValid _player
    (:Is%20Valid
      (bind _output_get (Variables|Default|SetDirToPlayer (Math|Vector|Normalize (- (Transformation|GetActorLocation _player) (Transformation|GetActorLocation)))))
      (if (>= (Math|Vector|DotProduct _output_get (Variables|Default|GetFacingVec)) (Variables|Default|Getvision))
        (bind _outhit (Collision|LineTraceByChannel (Transformation|GetActorLocation) (Transformation|GetActorLocation (Variables|Default|Getplayer)) "TraceTypeQuery1" false (Utilities|Array|MakeArray (Variables|Default|Getplayer)) "ForOneFrame"))
        (return (.bBlockingHit (Collision|BreakHitResult _outhit)) true)
        (else
          (return false false))))))

(fn LaserLengthTrace
  (params (Start :type Vector) (End :type Vector))
  (bind _laser (Variables|Default|Getlaser))
  (bind _returnvalue (Transformation|GetWorldLocation _laser))
  (bind (_outhit _returnvalue_2) (Collision|LineTraceByChannel Start End "TraceTypeQuery2" false 0 "ForDuration" true "(R=1.000000,G=0.000000,B=0.616345,A=1.000000)"))
  (Transformation|SetWorldScale3D (Variables|Default|Getlaser) (Math|Vector|MakeVector (Math|Float|SelectFloat (* (Math|Vector|Distance(Vector) _returnvalue (.Location (Collision|BreakHitResult _outhit))) 0.2) (* (Math|Vector|Distance(Vector) _returnvalue (.TraceEnd (Collision|BreakHitResult _outhit))) 0.2) _returnvalue_2) 1.0 1.0))
  (return (Math|Rotator|FindLookatRotation _returnvalue (.TraceEnd (Collision|BreakHitResult _outhit)))))