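; Sniper NPC whose laser sight serves as its line of vision and which awards score by player bounty when killed.
; In normal state, timelines drive a laser sweep while a timer runs cone and trace checks, feeding faked AI sight stimuli to the detection component.
; Other states turn the laser toward the player, with panic starting a shot timer.
; Shots are line traces with randomized aim offset and damage.
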(event Custom|ShootAtPlayer
  (bind _accuracyoffset (Variables|Default|GetAccuracyOffset))
  (bind _accuracydeviance (Variables|Default|GetAccuracyDeviance))
  ;[0.15 0.15 0.15 0.5] Sets the start rotation for tracking
  (Audio|PlaySoundatLocation "/Game/Audio/WeaponSounds/Sniper/CUE_Sniper.CUE_Sniper" (Transformation|GetActorLocation) "0, 0, 0" 1.0 1.0 0.0 0 0 0 0)
  (bind _outhit (Collision|LineTraceByChannel (Transformation|GetWorldLocation (Variables|Default|Getlaser)) (+ (Transformation|GetActorLocation (Variables|Default|Getplayer)) (Math|Vector|MakeVector (CallFunction|RandomwithDeviation _accuracyoffset _accuracydeviance) (CallFunction|RandomwithDeviation _accuracyoffset _accuracydeviance) (CallFunction|RandomwithDeviation _accuracyoffset _accuracydeviance))) "TraceTypeQuery2" false 0 "Persistent"))
  (Utilities|IsValid (.HitActor (Collision|BreakHitResult _outhit))
    (:Is%20Valid
      (Game|Damage|ApplyDamage (.HitActor (Collision|BreakHitResult _outhit)) (CallFunction|RandomwithDeviation (Variables|Default|GetBaseDamage) (Variables|Default|GetDamagedeviation)) 0 0))))

(event Custom|NormalVisionSweep
  ;[0.15 0.15 0.15 0.5] Normal State
  (Development|PrintString "Hello")
  (bind (_objinway _playerindot _returns_) (CallFunction|DetectPlayer))
  (if _returns_
    (if (or _objinway (not _playerindot))
      ;;[0.15 0.15 0.15 0.5] Lost Sight
      (Default|Sight (Variables|Default|GetBPC_Detection) (Variables|Default|Getplayer) (Utilities|Struct|MakeAIStimulus 0.0 0.0) (Variables|Default|GetSphere1) :!label _label)
      (Variables|Default|SetLOS false)
      (else
        ;;[0.15 0.15 0.15 0.5] Gained Sight - Boolean flag to prevent multiple calls of the Sight func.
        (if (not (Variables|Default|GetLOS))
          (Default|Sight (Variables|Default|GetBPC_Detection) (Variables|Default|Getplayer) (Utilities|Struct|MakeAIStimulus 0.0 0.0 -1.0 "340282346638528859811704183484516925440.000000,340282346638528859811704183484516925440.000000,340282346638528859811704183484516925440.000000" "340282346638528859811704183484516925440.000000,340282346638528859811704183484516925440.000000,340282346638528859811704183484516925440.000000" "None" true) (Variables|Default|GetSphere1))
          (Variables|Default|SetLOS true))))
    (else
      (goto _label))))

(event EventBeginPlay
  ;[0.15 0.15 0.15 0.5] Init
  (Utilities|FlowControl|Sequence
    (:then_0
      (bind _returnvalue (Actor|GetActorOfClass "/Game/Systems/Player/BP_Player.BP_Player_C"))
      (Utilities|IsValid _returnvalue
        (:Is%20Valid
          (Variables|Default|Setplayer _returnvalue))))
    (:then_1
      (|CallParentFunction))))

(event Collision|EventActorBeginOverlap
  (params (OtherActor :type Actor%20Object%20Reference)))

(event EventTick
  (params (DeltaSeconds :type Float%20%28single-precision%29))
  (bind _laser (Variables|Default|Getlaser))
  (bind _laser_2 (Variables|Default|Getlaser))
  (bind _returnvalue (Transformation|GetWorldLocation _laser))
  ;[0.15 0.15 0.15 0.5] Tick - Select based on SniperState
  (switch Utilities|FlowControl|Switch|SwitchonE_State (Variables|Default|GetcurrentState)
    (:NewEnumerator0
      ;[0.15 0.15 0.15 0.5] Normal Length Trace
      (CallFunction|LaserLengthTrace (Transformation|GetWorldLocation (Variables|Default|Getlaser)) (* (+ (Transformation|GetActorForwardVector) (Math|Transform|InverseTransformDirection (Transformation|GetActorTransform) (Variables|Default|GetOffset))) 1.5e+04))
      (CallFunction|OffsetLaser (Variables|Default|GetOffset))
      (Transformation|SetWorldRotation (Variables|Default|Getlaser) (Class|KismetMathLibrary|QuatRotator (Class|KismetMathLibrary|QuatSlerp (Math|Conversions|ToQuaternion(Rotator) (Math|Vector|GetForwardVector (Variables|Default|Getlaser))) (Math|Conversions|ToQuaternion(Rotator) (Variables|Default|GetFacingVec)) (* (Utilities|Time|GetWorldDeltaSeconds) (Variables|Default|GetCorrection%20Speed)))) false false))
    (:NewEnumerator1
      ;[0.15 0.15 0.15 0.5] Detecting/Panic Tracing
      (Transformation|SetWorldRotation (Variables|Default|Getlaser) (Math|Rotator|Lerp(Rotator) (Transformation|GetWorldRotation _laser_2) (Math|Rotator|FindLookatRotation (Transformation|GetWorldLocation _laser_2) (Transformation|GetActorLocation (Variables|Default|Getplayer))) (* (Utilities|Time|GetWorldDeltaSeconds) (Variables|Default|GetCorrection%20Speed))) false false :!label _label)
      (CallFunction|LaserLengthTrace _returnvalue (+ _returnvalue (* (Math|Vector|GetForwardVector _laser) 1.5e+04)))
      (CallFunction|CheckifPlayerBlocked))
    (:NewEnumerator3
      (goto _label))
    (:NewEnumerator2
      (goto _label))))

(event EventKill
  (params (Instigator :type Actor%20Object%20Reference))
  ;[0.15 0.15 0.15 0.5] Death
  (Utilities|FlowControl|Sequence
    (:then_0
      (Utilities|FlowControl|DoOnce false
        (:Completed
          (bind _e_bounty (CallFunction|GetBounty))
          (switch Utilities|FlowControl|Switch|SwitchonE_Bounty _e_bounty
            (:NewEnumerator0
              (CallFunction|AddScore 125.0 "Found you First!"))
            (:NewEnumerator1
              (CallFunction|AddScore 2.5e+02 "Missed Me!" :!label _label)
              (CallFunction|IncreaseBounty 25.0))
            (:NewEnumerator2
              (goto _label))
            (:NewEnumerator3
              (goto _label))))))
    (:then_1
      (|CallParentFunction Instigator))))

(event EventAlertState
  ;[0.15 0.15 0.15 0.5] Alert
  (Rendering|SetVisibility (Variables|Default|GetWantedPoster) false false)
  (Audio|Components|Audio|Stop (Variables|Default|GetVerticalSweep))
  (Audio|Components|Audio|Stop (Variables|Default|GetHorizontalSweep)))

(event EventNormalState
  ;[0.15 0.15 0.15 0.5] Normal State
  (Utilities|FlowControl|Sequence
    (:then_0
      ;;[0.15 0.15 0.15 0.5] Start Offset Timelines
      (Audio|Components|Audio|Play (Variables|Default|GetHorizontalSweep))
      (Audio|Components|Audio|Play (Variables|Default|GetVerticalSweep)))
    (:then_1
      (if (Utilities|Time|IsValidTimerHandle (Variables|Default|GetnormalVisionSweepTimer))
        (Utilities|Time|ClearandInvalidateTimerbyHandle (Variables|Default|GetnormalVisionSweepTimer)))
      (bind _returnvalue (Utilities|Time|SetTimerbyEvent (delegate Custom|NormalVisionSweep) 0.1 true))
      (Variables|Default|SetnormalVisionSweepTimer _returnvalue))
    (:then_2
      (Rendering|SetVisibility (Variables|Default|GetWantedPoster) false false))))

(event EventDetecting
  ;[0.15 0.15 0.15 0.5] Disables Offset Timelines
  (Utilities|FlowControl|Sequence
    (:then_0
      (Audio|Components|Audio|Stop (Variables|Default|GetVerticalSweep))
      (Audio|Components|Audio|Stop (Variables|Default|GetHorizontalSweep))
      (Development|PrintString "Hello"))
    (:then_1
      (bind _notifyname (Animation|Montage|PlayMontage (Variables|Character|GetMesh) "/Game/Art/SkeletalMesh/SniperNPC/AM_StartDetect.AM_StartDetect" 1.0 0.0 "None" false)
        (:OnNotifyBegin
          (switch name _notifyname
            (:ShowPaper
              (Rendering|SetVisibility (Variables|Default|GetWantedPoster) true false))))))))

(event EventPanicState
  ;[0.15 0.15 0.15 0.5] Sets the start rotation for tracking
  (Variables|Default|SetStartRot (Transformation|GetWorldRotation (Variables|Default|Getlaser)))
  (bind _returnvalue (Utilities|Time|SetTimerbyEvent (EventDispatchers|CreateEvent :!event Custom|ShootAtPlayer) (CallFunction|RandomwithDeviation (Variables|Default|GetShootInterval) (Variables|Default|GetShootIntervalDeviance)) true))
  (Variables|Default|SetShootTimer _returnvalue))

(fn ConstructionScript
  (|CallParentFunction)
  (Variables|Default|Setvision (Math|Trig|Cos(Degrees) (Variables|Default|GetFieldOfView)))
  (Development|PrintString "Hello"))

(fn OffsetLaser
  (params (Offset :type Vector))
  ;[0.5469 0.2822 0 0.5] Offset Laser
  (Variables|Default|SetFacingVec (Math|Vector|Normalize (+ (Transformation|GetActorForwardVector) (Math|Transform|InverseTransformDirection (Transformation|GetActorTransform) Offset)))))

(fn LaserLengthTrace
  (params (Start :type Vector) (End :type Vector))
  (bind _laser (Variables|Default|Getlaser))
  (bind _returnvalue (Transformation|GetWorldLocation _laser))
  (bind (_outhit _returnvalue_2) (Collision|LineTraceByChannel Start End "TraceTypeQuery2" false 0 "None" true "(R=1.000000,G=0.000000,B=0.616345,A=1.000000)"))
  (Transformation|SetWorldScale3D (Variables|Default|Getlaser) (Math|Vector|MakeVector (Math|Float|SelectFloat (* (Math|Vector|Distance(Vector) _returnvalue (.Location (Collision|BreakHitResult _outhit))) 0.2) (* (Math|Vector|Distance(Vector) _returnvalue (.TraceEnd (Collision|BreakHitResult _outhit))) 0.2) _returnvalue_2) 1.0 1.0))
  (return))

(fn DetectPlayer
  (bind _player (Variables|Default|Getplayer))
  (bind _vision (Variables|Default|Getvision))
  (Utilities|IsValid _player
    (:Is%20Valid
      (bind _output_get (Variables|Default|SetDirToPlayer (Math|Vector|Normalize (- (Transformation|GetActorLocation _player) (Transformation|GetActorLocation)))))
      (Development|PrintString (Utilities|String|Append (Utilities|String|ToString(Float) (Math|Vector|DotProduct _output_get (Math|Vector|GetForwardVector (Variables|Default|Getlaser)))) "             " (Utilities|String|ToString(Float) _vision)) true true "(R=1.000000,G=0.000000,B=0.129005,A=1.000000)" 2.0 "k")
      (if (>= (Math|Vector|DotProduct _output_get (Math|Vector|GetForwardVector (Variables|Default|Getlaser))) _vision)
        (bind _outhit (Collision|LineTraceByChannel (Transformation|GetActorLocation) (Transformation|GetActorLocation (Variables|Default|Getplayer)) "TraceTypeQuery1" false (Utilities|Array|MakeArray (Variables|Default|Getplayer)) "None"))
        (return (.bBlockingHit (Collision|BreakHitResult _outhit)) (>= (Math|Vector|DotProduct _output_get (Math|Vector|GetForwardVector (Variables|Default|Getlaser))) _vision) true)
        (else
          (return false false false))))))

(fn CheckifPlayerBlocked
  (bind _laser (Variables|Default|Getlaser))
  (bind _returnvalue (Transformation|GetWorldLocation _laser))
  (bind _returnvalue_2 (Collision|LineTraceByChannel _returnvalue (+ _returnvalue (* (Math|Vector|GetForwardVector _laser) 1.5e+03)) "TraceTypeQuery1" false (Utilities|Array|MakeArray (Variables|Default|Getplayer)) "None"))
  (return _returnvalue_2))

(fn RandomwithDeviation
  (params (Base :type Float%20%28double-precision%29) (Deviation :type Float%20%28double-precision%29))
  (return (+ Base (Math|Random|RandomFloatinRange (* Deviation -1.0) Deviation))))