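; Police NPC, a child of a shared NPC base, that patrols a spline path and shoots at the player when panicked.
; Panic approaches the player and starts a looping shot timer, which Decide clears before running parent logic.
; Shots are randomly offset line traces with varied damage, with player distance selecting aim angle and fire montage.
; Its death awards score or raises bounty and score modifier, depending on bounty level.
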(event Custom|Shoot
  (bind _returnvalue (Transformation|GetActorRotation))
  (bind _accuracydifference (Variables|Default|GetAccuracyDifference))
  (bind _damagedeviation (Variables|Default|GetdamageDeviation))
  (bind _returnvalue_2 (* _accuracydifference -1.0))
  ;[0.09905 0.1697 0.7188 0.5] Shoot
  (if (<= (Transformation|GetDistanceTo self (Variables|Default|GetPlayer)) (Variables|Default|GetGUN_RANGE))
    (bind _outhit (Collision|LineTraceByChannel (Transformation|GetActorLocation) (+ (Transformation|GetActorLocation (Variables|Default|GetPlayer)) (Math|Vector|MakeVector (Math|Random|RandomFloatinRange _returnvalue_2 _accuracydifference) (Math|Random|RandomFloatinRange _returnvalue_2 _accuracydifference) (Math|Random|RandomFloatinRange _returnvalue_2 _accuracydifference))) "TraceTypeQuery2" true 0 "Persistent"))
    (Transformation|SetActorRotation (Math|Rotator|MakeRotator (.roll _returnvalue) (.pitch _returnvalue) (.yaw (Math|Rotator|FindLookatRotation (Transformation|GetActorLocation) (Transformation|GetActorLocation (Variables|Default|GetPlayer))))))
    (CallFunction|Fire)
    (Utilities|IsValid (.HitActor (Collision|BreakHitResult _outhit))
      (:Is%20Valid
        (Game|Damage|ApplyDamage (.HitActor (Collision|BreakHitResult _outhit)) (+ (Variables|Default|GetdamageBase) (Math|Random|RandomFloatinRange (* _damagedeviation -1.0) _damagedeviation)) 0 0)))
    (else
      (CallFunction|Decide))))

(event Custom|ResetShoot
  ;[0.5729 0.2737 0 0.5] Panic
  (Utilities|FlowControl|DoOnce false) ; enters at Reset
)

(event Custom|Fire
  ;[0.02873 0.1399 0.3333 0.5] Shooting Anim Logic
  (if (<= (Transformation|GetDistanceTo self (Variables|Default|GetPlayer)) (Variables|Default|GetANGLE_THRESHOLD))
    (Animation|PlayAnimMontage "/Game/Art/SkeletalMesh/PoliceNPC/AM_Police_LowFire.AM_Police_LowFire" 1.0 "None")
    (else
      (Animation|PlayAnimMontage "/Game/Art/SkeletalMesh/PoliceNPC/AM_Police_Fire.AM_Police_Fire" 1.0 "None"))))

(event EventBeginPlay
  (bind _pathtofollow (Variables|Default|GetPathToFollow))
  (bind _returnvalue (Actor|GetActorOfClass "/Game/Systems/Player/BP_Player.BP_Player_C"))
  (Variables|Default|SetPlayer _returnvalue)
  (Utilities|IsValid _pathtofollow
    (:Is%20Valid
      (for _index (range 0 (Spline|GetNumberOfSplinePoints (Variables|/Game/Systems/NPC/NPC_Children/Police/BP_PolicePath.BP_PolicePath_C|GetSpline _pathtofollow)))
        (Utilities|Array|Add (Variables|Default|GetLocations) (Spline|GetLocationatSplinePoint (Variables|/Game/Systems/NPC/NPC_Children/Police/BP_PolicePath.BP_PolicePath_C|GetSpline (Variables|Default|GetPathToFollow)) _index "World"))))
    (:Is%20Not%20Valid
      _))
  (|CallParentFunction))

(event EventKill
  (params (Instigator :type Actor%20Object%20Reference))
  ;[0.6719 0.1365 0.6255 0.5] Kill Override
  (Utilities|FlowControl|Sequence
    (:then_0
      (bind _e_bounty (CallFunction|GetBounty))
      (switch Utilities|FlowControl|Switch|SwitchonE_Bounty _e_bounty
        (:NewEnumerator0
          (CallFunction|AddScore 2.5e+02 "Officer down!"))
        (:NewEnumerator1
          (CallFunction|IncreaseBounty 5e+01 :!label _label)
          (CallFunction|ApplyScoreModifier 0.25 "Most Wanted?"))
        (:NewEnumerator2
          (goto _label))
        (:NewEnumerator3
          (goto _label))))
    (:then_1
      (|CallParentFunction Instigator))))

(event EventTick
  (params (DeltaSeconds :type Float%20%28single-precision%29))
  ;[0.15 0 0.01661 0.5] Aiming (Bad code ahead don't @ me)
  (Utilities|IsValid (Variables|Default|GetPlayer)
    (:Is%20Valid
      (if (<= (Transformation|GetDistanceTo self (Variables|Default|GetPlayer)) (Variables|Default|GetANGLE_THRESHOLD))
        (Variables|Default|SetaimAngle 1e+02)
        (else
          (Variables|Default|SetaimAngle 0.0))))))

(event EventNormalState
  ;[0.455 0.6719 0.1063 0.5] NormalState
  (Utilities|IsValid (Variables|Default|GetPathToFollow)
    (:Is%20Valid
      (AI|AIMoveTo self (Utilities|Array|Get(acopy) (Variables|Default|GetLocations) (Variables|Default|Getindex)) 0 5.0 false
        (:OnSuccess
          (bind _result (Math|Integer|IncrementInt (Variables|Default|Getindex))
            (:%20%20
              (if (== _result (+ (Spline|GetNumberOfSplinePoints (Variables|/Game/Systems/NPC/NPC_Children/Police/BP_PolicePath.BP_PolicePath_C|GetSpline (Variables|Default|GetPathToFollow))) 1))
                (Variables|Default|Setindex 0))
              (CallFunction|Decide))))))))

(event EventPanicState
  ;[0.5729 0.2737 0 0.5] Panic
  (AI|AIMoveTo self "0, 0, 0" (Variables|Default|GetPlayer) 5e+02 false
    (:then
      (Utilities|FlowControl|DoOnce false
        (:Completed
          (bind _returnvalue (Utilities|Time|SetTimerbyEvent (EventDispatchers|CreateEvent :!event Custom|Shoot) (Variables|Default|GetshootCooldown) true))
          (Variables|Default|SetShootTimer _returnvalue))))))

(event EventDecide
  (bind _shoottimer (Variables|Default|GetShootTimer))
  ;[0.009116 0.7396 0.4675 0.5] Decidion
  (Utilities|FlowControl|Sequence
    (:then_0
      (CallFunction|ResetShoot)
      (if (Utilities|Time|IsValidTimerHandle _shoottimer)
        (Utilities|Time|ClearandInvalidateTimerbyHandle _shoottimer)))
    (:then_1
      (|CallParentFunction))))

(fn ConstructionScript
  (|CallParentFunction))